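; Test Blueprint that prints "Hello" from several events, with no evident gameplay purpose.
; On BeginPlay it calls Updatelogic, which starts a looping one-second timer that fires the get event to print.
; A separate TEST event runs GetAllActorsOfClass and a visibility multi line trace between Start and End, printing around the trace and leaving both results unused.
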(event `TEST`
  (params (Start :type "Vector Structure") (End :type "Vector Structure"))
  (`GameplayStatics.GetAllActorsOfClass` null)
  (`KismetSystemLibrary.PrintString` "Hello")
  (`KismetSystemLibrary.LineTraceMulti` Start End "TraceTypeQuery1")
  (`KismetSystemLibrary.PrintString` "Hello"))

(event `self.ReceiveBeginPlay`
  (`self.Updatelogic`)
  (`KismetSystemLibrary.PrintString` "Hello"))

(event `Updatelogic`
  (`KismetSystemLibrary.K2_SetTimer` null "get" 1.0 true))

(event `get`
  (`KismetSystemLibrary.PrintString` "Hello"))

(fn `UserConstructionScript`)