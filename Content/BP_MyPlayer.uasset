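; BP_MyPlayer is a player Blueprint with basic movement and look controls plus debug-style LAN multiplayer hosting and joining.
; Axis inputs drive movement along the actor's forward and right vectors, and controller yaw and pitch.
; X creates a LAN session and opens MainLevel as a listen server.
; Z searches LAN sessions and joins the first result without checking for an empty list, printing status messages along the way.
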(event `InputAxis|Turn`
  (params (AxisValue :type "Float (single-precision)"))
  (`self.AddControllerYawInput` AxisValue))

(event `InputAxis|MoveForward`
  (params (AxisValue :type "Float (single-precision)"))
  (`self.AddMovementInput` (`self.GetActorForwardVector`) AxisValue))

(event `InputAxis|LookUp`
  (params (AxisValue :type "Float (single-precision)"))
  (`self.AddControllerPitchInput` AxisValue))

(event `InputAxis|MoveRight`
  (params (AxisValue :type "Float (single-precision)"))
  (`self.AddMovementInput` (`self.GetActorRightVector`) AxisValue))

(event `Key|X`
  (params (Key :type "Key Structure"))
  (:`Pressed`
    (`KismetSystemLibrary.PrintString` "CREATING SESSION!")
    (`CreateSessionCallbackProxy.CreateSession` (`GameplayStatics.GetPlayerController` 0) 10 true
      (:`OnSuccess`
        (`KismetSystemLibrary.PrintString` "CREATED SESSION!")
        (`GameplayStatics.OpenLevelBySoftObjectPtr` "/Game/MainLevel.MainLevel" true "listen")))))

(event `Key|Z`
  (params (Key :type "Key Structure"))
  (bind _returnvalue (`GameplayStatics.GetPlayerController` 0))
  (:`Pressed`
    (`KismetSystemLibrary.PrintString` "FINDING SESSION!")
    (bind _results (`FindSessionsCallbackProxy.FindSessions` _returnvalue 100 true)
      (:`OnSuccess`
        (`JoinSessionCallbackProxy.JoinSession` _returnvalue (`|GetArrayItem` _results)
          (:`OnSuccess`
            (`KismetSystemLibrary.PrintString` "JOINED SESSION!"))
          (:`OnFailure`
            (`KismetSystemLibrary.PrintString` "FAILED JOINED"))))
      (:`OnFailure`
        (`KismetSystemLibrary.PrintString` "FAILED SESSION!")))))

(fn `UserConstructionScript`)