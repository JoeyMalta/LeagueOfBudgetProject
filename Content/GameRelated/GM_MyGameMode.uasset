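; Game mode that auto-balances joining players between Blue and Red teams.
; PostLogin adds the player to Red when Blue is larger, otherwise Blue, and copies the team to controller and player state.
; The returned array index becomes the controller's PlayerID.
; Logout removes the controller from TeamRed if TeamBlue contains it, otherwise from TeamBlue, so the selection appears inverted.
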(event `self.K2_PostLogin`
  (params (NewPlayer :type "PlayerController Object Reference"))
  (bind _returnvalue (> (`KismetArrayLibrary.Array_Length` (`self.TeamBlue`)) (`KismetArrayLibrary.Array_Length` (`self.TeamRed`))))
  (bind _aspc_player_controller (cast `/Game/PlayerRelated/PC_PlayerController` NewPlayer))
  (bind _output_get (set `/Game/PlayerRelated/PC_PlayerController.currentTeam` (select `bool` _returnvalue :`false` "NewEnumerator0" :`true` "NewEnumerator1" :!type "/Game/PlayerRelated/TeamSystem/ENUM_Teams Enum") _aspc_player_controller))
  (set `/Game/PlayerRelated/PS_MyPlayerState.PlayerTeam` _output_get (cast `/Game/PlayerRelated/PS_MyPlayerState` (`Controller.PlayerState` NewPlayer) :!pure true))
  (bind _returnvalue_2 (`KismetArrayLibrary.Array_Add` (select `bool` _returnvalue :`false` (`self.TeamBlue`) :`true` (`self.TeamRed`)) NewPlayer))
  (set `/Game/PlayerRelated/PC_PlayerController.PlayerID` _returnvalue_2 _aspc_player_controller))

(event `self.K2_OnLogout`
  (params (ExitingController :type "Controller Object Reference"))
  (bind _asplayer_controller (cast `PlayerController` ExitingController))
  (`KismetArrayLibrary.Array_RemoveItem` (select `bool` (`KismetArrayLibrary.Array_Contains` (`self.TeamBlue`) _asplayer_controller) :`false` (`self.TeamBlue`) :`true` (`self.TeamRed`)) _asplayer_controller))

(fn `UserConstructionScript`)