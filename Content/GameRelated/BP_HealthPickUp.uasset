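; BP_HealthPickUp is a health pickup that heals a player who touches it and then disappears.
; On BeginPlay it caches its owner as the BP_HealthSpawner that manages it.
; Box overlap forwards the other actor to an SRV-prefixed event, which adds a fixed amount to BP_MyPlayer's health component, clears the spawner's pickup reference and destroys the pickup.
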(event `self.ReceiveBeginPlay`
  (bind _asbp_health_spawner (cast `/Game/GameRelated/BP_HealthSpawner` (`self.GetOwner`)))
  (set `self.BP_HealthSpawner` _asbp_health_spawner))

(event `self.Box.OnComponentBeginOverlap`
  (params (OverlappedComponent :type "PrimitiveComponent Object Reference") (OtherActor :type "Actor Object Reference") (OtherComp :type "PrimitiveComponent Object Reference") (OtherBodyIndex :type Integer) (bFromSweep :type Boolean) (SweepResult :type "HitResult Structure (by ref)"))
  (`self.SRV_overlapPlayer` OtherActor))

(event `SRV_overlapPlayer`
  (params (BP_MyPlayer :type "Actor Object Reference"))
  (bind _asbp_my_player (cast `/Game/PlayerRelated/BP_MyPlayer` BP_MyPlayer))
  (`/Game/PlayerRelated/PlayerComponents/BP_PlayerHealth.addHealth` (`/Game/PlayerRelated/BP_MyPlayer.BP_PlayerHealth` _asbp_my_player) 20.0)
  (set `/Game/GameRelated/BP_HealthSpawner.BP_HealthPickUp` null (`self.BP_HealthSpawner`))
  (`self.K2_DestroyActor`))

(fn `UserConstructionScript`)