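; BP_Tower is a team-colored defensive tower that fires on enemy characters and is destroyed when its health runs out.
; Its construction script applies blue or red materials and tags the actor with its team.
; Characters entering the sphere with the enemy team tag trigger a single BP_TowerBullet spawn at the arrow, with that character set as Owner.
; Damage feeds the player health component, whose death event destroys the tower.
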(event `self.Sphere.OnComponentBeginOverlap`
  (params (OverlappedComponent :type "PrimitiveComponent Object Reference") (OtherActor :type "Actor Object Reference") (OtherComp :type "PrimitiveComponent Object Reference") (OtherBodyIndex :type Integer) (bFromSweep :type Boolean) (SweepResult :type "HitResult Structure (by ref)"))
  (`self.Overlap` OtherActor))

(event `Overlap`
  (params (actor :type "Actor Object Reference"))
  (bind _ascharacter (cast `Character` actor))
  (if (`KismetArrayLibrary.Array_Contains` (`Actor.Tags` _ascharacter) (`KismetStringLibrary.Conv_StringToName` (`|GetEnumeratorNameAsString` (`self.enemyTeam`))))
    (`|SpawnActorFromClass` "/Game/GameRelated/BP_TowerBullet.BP_TowerBullet_C" (`KismetMathLibrary.MakeTransform` (`SceneComponent.K2_GetComponentLocation` (`self.Arrow`)) (struct) (0.2 0.2 0.2)) "AlwaysSpawn" "OverrideRootScale" _ascharacter null null)))

(event `self.ReceiveAnyDamage`
  (params (Damage :type "Float (single-precision)") (DamageType :type "DamageType Object Reference") (InstigatedBy :type "Controller Object Reference") (DamageCauser :type "Actor Object Reference"))
  (bind _newhealth (`/Game/PlayerRelated/PlayerComponents/BP_PlayerHealth.removeHealth` (`self.BP_PlayerHealth`) Damage))
  (`KismetSystemLibrary.PrintString` (`KismetStringLibrary.Conv_DoubleToString` _newhealth) true true (struct :`R` 0.014378 :`G` 1.0 :`A` 1.0)))

(event `self.Sphere.OnComponentEndOverlap`
  (params (OverlappedComponent :type "PrimitiveComponent Object Reference") (OtherActor :type "Actor Object Reference") (OtherComp :type "PrimitiveComponent Object Reference") (OtherBodyIndex :type Integer))
  (`self.endOverlap` OtherActor))

(event `endOverlap`
  (params (actor :type "Actor Object Reference"))
  (cast `/Game/PlayerRelated/BP_MyPlayer` actor)
  (set `self.inRange` false))

(event `self.BP_PlayerHealth.Event_isDead`
  (`self.K2_DestroyActor`))

(fn `UserConstructionScript`
  (bind _currentteam (`self.currentTeam`))
  (bind _tags (`self.Tags`))
  (bind _returnvalue (`|GetEnumeratorNameAsString` _currentteam))
  (switch `/Game/PlayerRelated/TeamSystem/ENUM_Teams` _currentteam
    (:`NewEnumerator0`
      (`PrimitiveComponent.SetMaterial` (`self.tower`) 0 "/Game/Assets/Materials/M_BlueMaterial.M_BlueMaterial")
      (`PrimitiveComponent.SetMaterial` (`self.Cone`) 0 "/Game/Assets/Materials/M_BlueMaterial.M_BlueMaterial")
      (`KismetArrayLibrary.Array_Add` _tags (`KismetStringLibrary.Conv_StringToName` _returnvalue)))
    (:`NewEnumerator1`
      (`PrimitiveComponent.SetMaterial` (`self.Cone`) 0 "/Game/Assets/Materials/M_RedMaterial.M_RedMaterial")
      (`PrimitiveComponent.SetMaterial` (`self.tower`) 0 "/Game/Assets/Materials/M_RedMaterial.M_RedMaterial")
      (`KismetArrayLibrary.Array_Add` _tags (`KismetStringLibrary.Conv_StringToName` _returnvalue)))))