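; BP_PlayerBullet is a homing projectile that seeks its own owner and damages it on contact.
; On BeginPlay, an SRV-prefixed event sets the projectile movement's homing target to an Arrow component on the owner.
; Sphere overlaps feed a second SRV event, which applies fixed damage and destroys the bullet only when the overlapped actor is a Character and is that owner.
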(event `self.ReceiveBeginPlay`
  (`self.SRV_projectile`))

(event `SRV_projectile`
  (set `ProjectileMovementComponent.HomingTargetComponent` (`self.GetComponentByClass` (`self.GetOwner`) "/Script/Engine.ArrowComponent") (`self.ProjectileMovement`)))

(event `SRV_Overlap`
  (params (A :type "Object Object Reference"))
  (bind _ascharacter (cast `Character` A))
  (if (== A (`self.GetOwner`))
    (`GameplayStatics.ApplyDamage` _ascharacter 15.0 null self)
    (`self.K2_DestroyActor`)))

(event `self.Sphere1.OnComponentBeginOverlap`
  (params (OverlappedComponent :type "PrimitiveComponent Object Reference") (OtherActor :type "Actor Object Reference") (OtherComp :type "PrimitiveComponent Object Reference") (OtherBodyIndex :type Integer) (bFromSweep :type Boolean) (SweepResult :type "HitResult Structure (by ref)"))
  (`self.SRV_Overlap` OtherActor))

(fn `UserConstructionScript`)