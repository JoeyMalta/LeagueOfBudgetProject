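; BP_TowerBullet is a homing tower projectile that damages the character set as its Owner, so the Owner serves as the target rather than the shooter.
; BeginPlay calls a server-named projectile event, which points ProjectileMovement's homing target at the Owner's ArrowComponent; the event's player parameter is unused.
; A Sphere1 overlap applies fixed damage and destroys the bullet only when the overlapping Character is that Owner.
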(event `self.ReceiveBeginPlay`
  (`self.SRV_projectile` null))

(event `SRV_projectile`
  (params (BP_MyPlayer :type "/Game/PlayerRelated/BP_MyPlayer Object Reference"))
  (set `ProjectileMovementComponent.HomingTargetComponent` (`self.GetComponentByClass` (`self.GetOwner`) "/Script/Engine.ArrowComponent") (`self.ProjectileMovement`)))

(event `self.Sphere1.OnComponentBeginOverlap`
  (params (OverlappedComponent :type "PrimitiveComponent Object Reference") (OtherActor :type "Actor Object Reference") (OtherComp :type "PrimitiveComponent Object Reference") (OtherBodyIndex :type Integer) (bFromSweep :type Boolean) (SweepResult :type "HitResult Structure (by ref)"))
  (bind _ascharacter (cast `Character` OtherActor))
  (if (== _ascharacter (`self.GetOwner`))
    (`GameplayStatics.ApplyDamage` _ascharacter 5.0 null self)
    (`self.K2_DestroyActor`)))

(fn `UserConstructionScript`)