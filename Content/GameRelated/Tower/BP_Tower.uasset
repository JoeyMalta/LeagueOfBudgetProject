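; BP_Tower is a team-based defensive tower that shoots at enemy characters entering its range sphere.
; Overlap locks one target and starts a looping "fire" timer that spawns BP_TowerBullet at the arrow, passing the target as Owner.
; Without a target, fire rescans overlapping melee minions for enemies.
; A health component takes damage and destroys the tower on death, a widget shows health, and the construction script sets team material.
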(event `self.ReceiveBeginPlay`
  (bind _aswb_aihealth (cast `/Game/GameRelated/ArtificialIntelligence/WB_AIHealth` (`WidgetComponent.GetUserWidgetObject` (`self.Widget`))))
  (`/Game/GameRelated/ArtificialIntelligence/WB_AIHealth.Init` _aswb_aihealth self))

(event `self.Sphere.OnComponentBeginOverlap`
  (params (OverlappedComponent :type "PrimitiveComponent Object Reference") (OtherActor :type "Actor Object Reference") (OtherComp :type "PrimitiveComponent Object Reference") (OtherBodyIndex :type Integer) (bFromSweep :type Boolean) (SweepResult :type "HitResult Structure (by ref)"))
  (`self.Overlap` OtherActor))

(event `Overlap`
  (params (actor :type "Actor Object Reference"))
  (`/Engine/EditorBlueprintResources/StandardMacros.IsValid` (`self.Other Actor`)
    (:`Is Not Valid`
      (bind _ascharacter (cast `Character` actor))
      (bind _current (message `/Game/GameRelated/ArtificialIntelligence/BI_AISettings.getcurrentTeam` _ascharacter))
      (if (`|EnumEquality` _current (`self.enemyTeam`))
        (set `self.Other Actor` _ascharacter)
        (`KismetSystemLibrary.K2_SetTimer` null "fire" 1.0 true)))))

(event `self.ReceiveAnyDamage`
  (params (Damage :type "Float (single-precision)") (DamageType :type "DamageType Object Reference") (InstigatedBy :type "Controller Object Reference") (DamageCauser :type "Actor Object Reference"))
  (bind _newhealth (`/Game/PlayerRelated/PlayerComponents/BP_PlayerHealth.removeHealth` (`self.BP_PlayerHealth`) Damage))
  (`KismetSystemLibrary.PrintString` (`KismetStringLibrary.Conv_DoubleToString` _newhealth) true true (struct :`R` 0.014378 :`G` 1.0 :`A` 1.0)))

(event `fire`
  (`/Engine/EditorBlueprintResources/StandardMacros.IsValid` (`self.Other Actor`)
    (:`Is Valid`
      (`|SpawnActorFromClass` "/Game/GameRelated/Tower/BP_TowerBullet.BP_TowerBullet_C" (`KismetMathLibrary.MakeTransform` (`SceneComponent.K2_GetComponentLocation` (`self.Arrow`)) (struct) (0.2 0.2 0.2)) "AlwaysSpawn" "OverrideRootScale" (`self.Other Actor`) null null))
    (:`Is Not Valid`
      (for _array_element (`PrimitiveComponent.GetOverlappingActors` (`self.Sphere`) "/Game/GameRelated/ArtificialIntelligence/AI_MeleeMinion.AI_MeleeMinion_C")
        (bind _current (message `/Game/GameRelated/ArtificialIntelligence/BI_AISettings.getcurrentTeam` _array_element))
        (if (`|EnumEquality` _current (`self.enemyTeam`))
          (set `self.Other Actor` _array_element)
          (else
            (`KismetSystemLibrary.K2_ClearTimer` null "fire")))))))

(event `self.Sphere.OnComponentEndOverlap`
  (params (OverlappedComponent :type "PrimitiveComponent Object Reference") (OtherActor :type "Actor Object Reference") (OtherComp :type "PrimitiveComponent Object Reference") (OtherBodyIndex :type Integer))
  (`self.endOverlap` OtherActor))

(event `endOverlap`
  (params (actor :type "Actor Object Reference"))
  (if (== actor (`self.Other Actor`))
    (set `self.Other Actor` null)
    (set `self.inRange` false)))

(event `self.BP_PlayerHealth.Event_isDead`
  (`self.K2_DestroyActor`))

(fn `getcurrentTeam`
  (returns (current :type "/Game/PlayerRelated/TeamSystem/ENUM_Teams Enum"))
  (return (`self.currentTeam`)))

(fn `getenemyTeam`
  (returns (enemy :type "/Game/PlayerRelated/TeamSystem/ENUM_Teams Enum"))
  (return (`self.enemyTeam`)))

(fn `UserConstructionScript`
  (bind _tower (`self.tower`))
  (switch `/Game/PlayerRelated/TeamSystem/ENUM_Teams` (`self.currentTeam`)
    (:`NewEnumerator0`
      (`PrimitiveComponent.SetMaterial` _tower 3 "/Game/Assets/Tower/M_Tower_1.M_Tower_1"))
    (:`NewEnumerator1`
      (`PrimitiveComponent.SetMaterial` _tower 3 "/Game/Assets/Tower/M_Tower_7.M_Tower_7"))))