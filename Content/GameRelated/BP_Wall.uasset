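; BP_Wall is a short-lived team-colored wall actor that destroys itself about a second after its color is set.
; SRV_ChangeColor picks the Cube's material from the Team value, Blue or Red, then waits briefly and destroys the actor.
; Both the Construction Script and BeginPlay call this event, so coloring and timed removal share one path.
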(event `self.ReceiveBeginPlay`
  (`self.SRV_ChangeColor`))

(event `SRV_ChangeColor`
  (bind _cube (`self.Cube`))
  (switch `/Game/PlayerRelated/TeamSystem/ENUM_Teams` (`self.team`)
    (:`NewEnumerator0`
      (`PrimitiveComponent.SetMaterial` _cube 0 "/Game/Assets/Materials/M_Wall_2.M_Wall_2"))
    (:`NewEnumerator1`
      (`PrimitiveComponent.SetMaterial` _cube 0 "/Game/Assets/Materials/M_Wall.M_Wall")))
  (`KismetSystemLibrary.Delay` 1.0)
  (`self.K2_DestroyActor`))

(fn `UserConstructionScript`
  (`self.SRV_ChangeColor`))