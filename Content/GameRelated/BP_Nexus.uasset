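; Team nexus actor whose destruction triggers a game-end message for its team.
; The construction script sets the mesh materials from CurrentTeam, and getters expose the current and enemy teams.
; BeginPlay binds a health widget to the actor.
; AnyDamage subtracts health through the player health component, then sends the message and destroys the actor once it is dead.
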(event `self.ReceiveBeginPlay`
  (bind _aswb_aihealth (cast `/Game/GameRelated/ArtificialIntelligence/WB_AIHealth` (`WidgetComponent.GetUserWidgetObject` (`self.Widget`))))
  (`/Game/GameRelated/ArtificialIntelligence/WB_AIHealth.Init` _aswb_aihealth self))

(event `self.ReceiveAnyDamage`
  (params (Damage :type "Float (single-precision)") (DamageType :type "DamageType Object Reference") (InstigatedBy :type "Controller Object Reference") (DamageCauser :type "Actor Object Reference"))
  (bind _bp_playerhealth (`self.BP_PlayerHealth`))
  (`/Game/PlayerRelated/PlayerComponents/BP_PlayerHealth.removeHealth` _bp_playerhealth Damage)
  (if (`/Game/PlayerRelated/PlayerComponents/BP_PlayerHealth.isDead` _bp_playerhealth)
    (message `/Game/GameRelated/I_GameOver.GameEnds` self (`self.currentTeam`) self)
    (`self.K2_DestroyActor`)))

(fn `getcurrentTeam`
  (returns (current :type "/Game/PlayerRelated/TeamSystem/ENUM_Teams Enum"))
  (return (`self.currentTeam`)))

(fn `getenemyTeam`
  (returns (enemy :type "/Game/PlayerRelated/TeamSystem/ENUM_Teams Enum"))
  (return (`self.EnemyTeam`)))

(fn `UserConstructionScript`
  (bind _nexus (`self.nexus`))
  (switch `/Game/PlayerRelated/TeamSystem/ENUM_Teams` (`self.currentTeam`)
    (:`NewEnumerator0`
      (`PrimitiveComponent.SetMaterial` _nexus 0 "/Game/Assets/Materials/M_BlueMaterial.M_BlueMaterial"))
    (:`NewEnumerator1`
      (`PrimitiveComponent.SetMaterial` _nexus 0 "/Game/Assets/Nexus/nexus_9.nexus_9")
      (`PrimitiveComponent.SetMaterial` _nexus 1 "/Game/Assets/Nexus/nexus_7.nexus_7")
      (`PrimitiveComponent.SetMaterial` _nexus 2 "/Game/Assets/Nexus/nexus_8.nexus_8"))))