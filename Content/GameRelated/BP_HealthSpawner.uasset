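; BP_HealthSpawner is a networked spawner that places a health pickup just above its own location.
; On BeginPlay the authority starts a short timer that calls SRV_SpawnHealth, which spawns BP_HealthPickUp with itself as owner and stores the reference.
; The reference's RepNotify restarts that timer whenever it fires with an invalid pickup, requesting a respawn, though the spawn itself runs only with authority.
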(event `self.ReceiveBeginPlay`
  (`/Engine/EditorBlueprintResources/ActorMacros.Switch Has Authority`
    (:`Authority`
      (`KismetSystemLibrary.K2_SetTimer` null "SRV_SpawnHealth" 3.0))))

(event `SRV_SpawnHealth`
  (`/Engine/EditorBlueprintResources/ActorMacros.Switch Has Authority`
    (:`Authority`
      (bind _returnvalue (`|SpawnActorFromClass` "/Game/GameRelated/BP_HealthPickUp.BP_HealthPickUp_C" (`KismetMathLibrary.MakeTransform` (`KismetMathLibrary.MakeVector` (.x (`self.K2_GetActorLocation`)) (.y (`self.K2_GetActorLocation`)) (+ (.z (`self.K2_GetActorLocation`)) 100.0))) "AdjustIfPossibleButAlwaysSpawn" "OverrideRootScale" self null))
      (set `self.BP_HealthPickUp` _returnvalue))))

(fn `OnRep_BP_HealthPickUp`
  (`self.BP_HealthPickUp`
    (:`then`)
    (:`else`
      (`KismetSystemLibrary.K2_SetTimer` null "SRV_SpawnHealth" 3.0))))

(fn `UserConstructionScript`)