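; Player bullet projectile that damages characters, towers and the nexus on overlap.
; BeginPlay calls an SRV-prefixed event that sets the projectile's homing target to an ArrowComponent on its owner.
; Sphere overlaps route through another SRV event: characters take fixed damage only if they are the bullet's owner, while towers and the nexus take random damage in separate ranges.
; The bullet destroys itself after dealing damage.
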(event `self.ReceiveBeginPlay`
  (`self.SRV_projectile`))

(event `SRV_projectile`
  (set `ProjectileMovementComponent.HomingTargetComponent` (`self.GetComponentByClass` (`self.GetOwner`) "/Script/Engine.ArrowComponent") (`self.ProjectileMovement`)))

(event `SRV_Overlap`
  (params (A :type "Object Object Reference"))
  (bind _ascharacter (cast `Character` A)
    (:`then`
      (if (== A (`self.GetOwner`))
        (`GameplayStatics.ApplyDamage` _ascharacter 5.0 null (`self.fromPlayer`))
        (`self.K2_DestroyActor` :!label _label)))
    (:`CastFailed`
      (bind _asbp_tower (cast `/Game/GameRelated/Tower/BP_Tower` A)
        (:`then`
          (`GameplayStatics.ApplyDamage` _asbp_tower (`KismetMathLibrary.RandomFloatInRange` 50.0 100.0) null self)
          (goto _label))
        (:`CastFailed`
          (bind _asbp_nexus (cast `/Game/GameRelated/BP_Nexus` A))
          (`GameplayStatics.ApplyDamage` _asbp_nexus (`KismetMathLibrary.RandomFloatInRange` 1.0 5.0) null self)
          (goto _label))))))

(event `self.Sphere1.OnComponentBeginOverlap`
  (params (OverlappedComponent :type "PrimitiveComponent Object Reference") (OtherActor :type "Actor Object Reference") (OtherComp :type "PrimitiveComponent Object Reference") (OtherBodyIndex :type Integer) (bFromSweep :type Boolean) (SweepResult :type "HitResult Structure (by ref)"))
  (`self.SRV_Overlap` OtherActor))

(fn `UserConstructionScript`)