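; Temporary camera pawn that the player controls until it hands over to a BP_MyPlayer character.
; MoveForward and MoveRight axes offset it locally by MoveSpeed.
; Seven seconds after BeginPlay it spawns BP_MyPlayer at the PC_PlayerController's PlayerSpawn, has the controller possess it, then destroys itself.
; Screen-edge scrolling, cursor-follow movement and greyscale post-process are leftover experiments, disconnected from the live event flow.
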(event `InputAxis|MoveForward`
  (params (AxisValue :type "Float (single-precision)"))
  (`self.K2_AddActorLocalOffset` (`KismetMathLibrary.MakeVector` (* AxisValue (`self.MoveSpeed`)))))

(event `InputAxis|MoveRight`
  (params (AxisValue :type "Float (single-precision)"))
  (`self.K2_AddActorLocalOffset` (`KismetMathLibrary.MakeVector` 0.0 (* AxisValue (`self.MoveSpeed`)))))

(event `self.ReceiveBeginPlay`
  (bind _returnvalue (`self.GetController`))
  (bind _playerspawn (`/Game/PlayerRelated/PC_PlayerController.PlayerSpawn` (cast `/Game/PlayerRelated/PC_PlayerController` _returnvalue :!pure true)))
  (`KismetSystemLibrary.Delay` 7.0)
  (bind _returnvalue_2 (`|SpawnActorFromClass` "/Game/PlayerRelated/BP_MyPlayer.BP_MyPlayer_C" (`KismetMathLibrary.MakeTransform` (`self.K2_GetActorLocation` _playerspawn) (`self.K2_GetActorRotation` _playerspawn)) "AlwaysSpawn" "OverrideRootScale" null null))
  (`Controller.Possess` _returnvalue _returnvalue_2)
  (`self.K2_DestroyActor`))

(event `LCL`)

(event `moveto`)

(event `InputAction|RMB`
  (params (Key :type "Key Structure"))
  ;[1 1 1] Rightmouse button - move player
)

(event `SRV_spawnAsPlayer`)

(event `InputAction|RMB`
  (params (Key :type "Key Structure")))

(event `CustomEvent_0`
  (bind _returnvalue (`WidgetLayoutLibrary.GetMousePositionOnViewport`))
  (bind (_x _y) (`KismetMathLibrary.BreakVector2D` _returnvalue))
  (bind _output_get (set `self.Impact Point` (`KismetMathLibrary.MakeVector` _x _y 2000.0)))
  (`SceneComponent.K2_SetWorldLocation` (`self.DefaultSceneRoot`) (`KismetMathLibrary.MakeVector` (.x _output_get) (.y _output_get) (.z _output_get)) false false))

(event `InputAction|RMB`
  (params (Key :type "Key Structure")))

(event `InputAxisKey|MouseX`
  (params (AxisValue :type "Float (single-precision)")))

(event `InputAxisKey|MouseY`
  (params (AxisValue :type "Float (single-precision)")))

(event `testing`)

(fn `OnRep_BP_MyPlayer`)

(fn `setPostProcessToDefault`
  (`|VariableSetRef` (`.ColorSaturation` (break `PostProcessSettings` (`PostProcessComponent.Settings` (`self.PostProcess`)))) (`KismetMathLibrary.MakeVector4` 1.0 1.0 1.0 1.0)))

(fn `setPostProcessToGrey`
  (`|VariableSetRef` (`.ColorSaturation` (break `PostProcessSettings` (`PostProcessComponent.Settings` (`self.PostProcess`)))) (`KismetMathLibrary.MakeVector4` 0.1 0.1 0.1 1.0)))

(fn `UserConstructionScript`)