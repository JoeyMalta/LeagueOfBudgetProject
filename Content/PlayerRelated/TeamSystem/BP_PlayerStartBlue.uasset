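; Team player start actor that marks a spawn point as belonging to Blue or Red Team.
; The construction script switches on the Team variable, sets the billboard to the green icon for Blue or the red icon for Red, and adds the team's enum name to the actor's Tags.
; It has no runtime logic, as all event graph nodes are disabled stubs.
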(fn `UserConstructionScript`
  (bind _returnvalue (`|GetEnumeratorNameAsString` (`self.Team`)))
  (switch `/Game/PlayerRelated/TeamSystem/ENUM_Teams` (`self.Team`)
    (:`NewEnumerator0`
      (`BillboardComponent.SetSprite` (`self.Billboard`) "/Engine/EngineResources/AICON-Green.AICON-Green")
      (`KismetArrayLibrary.Array_Add` (`self.Tags`) (`KismetStringLibrary.Conv_StringToName` _returnvalue)))
    (:`NewEnumerator1`
      (`BillboardComponent.SetSprite` (`self.Billboard`) "/Engine/EngineResources/AICON-Red.AICON-Red")
      (`KismetArrayLibrary.Array_Add` (`self.Tags`) (`KismetStringLibrary.Conv_StringToName` _returnvalue)))))