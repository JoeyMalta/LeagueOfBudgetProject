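; BP_TeamStart is a team start marker, tagged with the name of the team set in its EnumsTeams variable.
; The construction script adds that tag and sets the billboard sprite by team: a green icon for Blue, a red one for Red.
; The Initialize event only clears the tags; the event graph's node to re-add the team tag is unconnected, and BeginPlay is empty.
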(event `self.ReceiveBeginPlay`)

(event `Initialize`
  (`KismetArrayLibrary.Array_Clear` (`self.Tags`)))

(fn `UserConstructionScript`
  (bind _billboard (`self.Billboard`))
  (`KismetArrayLibrary.Array_Add` (`self.Tags`) (`KismetStringLibrary.Conv_StringToName` (`|GetEnumeratorNameAsString` (`self.Enums_Teams`))))
  (switch `/Game/PlayerRelated/TeamSystem/ENUM_Teams` (`self.Enums_Teams`)
    (:`NewEnumerator0`
      (`BillboardComponent.SetSprite` _billboard "/Engine/EngineResources/AICON-Green.AICON-Green"))
    (:`NewEnumerator1`
      (`BillboardComponent.SetSprite` _billboard "/Engine/EngineResources/AICON-Red.AICON-Red"))))