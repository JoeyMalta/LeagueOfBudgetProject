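; Player pawn for a multiplayer game with click-to-move, wheel-zoom camera and health.
; Right-click stores the cursor hit point, and a looping timer feeds movement input toward it; Tick eases spring arm zoom.
; Damage drains BPPlayerHealth; death spawns and possesses a BP_Spectator, then destroys the pawn, while Q spectates via player controller 0.
; After BeginPlay, a server-to-multicast chain assigns PlayerStates to name widgets; X/Z host or join through console commands.
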(event `self.ReceiveBeginPlay`
  ;[1 1 1] Player movement - right mouse button
  (`KismetSystemLibrary.Delay` 1.0)
  (`self.SRV_playerMovement`))

(event `SRV_playerMovement`
  ;[1 1 1] Player movement - right mouse button
  (`self.MC_playerMovement`))

(event `MC_playerMovement`
  ;[1 1 1] Player movement - right mouse button
  (bind _outactors (`GameplayStatics.GetAllActorsOfClass` "BP_MyPlayer_C"))
  (for _array_element _outactors
    (bind _aswb_player_name (cast `/Game/Widgets/WB_PlayerName` (`WidgetComponent.GetUserWidgetObject` (`/Game/PlayerRelated/BP_MyPlayer.WB_PlayerNameComponent` _array_element))))
    (set `/Game/Widgets/WB_PlayerName.PlayerState` (`Pawn.PlayerState` _array_element) _aswb_player_name)))

(event `InputAction|RMB`
  (params (Key :type "Key Structure"))
  (bind (_hitresult _returnvalue) (`PlayerController.GetHitResultUnderCursorByChannel` (`GameplayStatics.GetPlayerController` 0) "TraceTypeQuery1" true))
  ;[1 1 1] Rightmouse button - move player
  (:`Pressed`
    (if _returnvalue
      (set `self.Impact Point` (`.ImpactPoint` (`GameplayStatics.BreakHitResult` _hitresult)))
      (`KismetSystemLibrary.K2_SetTimerDelegate` (delegate `UpdateMovement`) 0.01 true))))

(event `UpdateMovement`
  (bind _returnvalue (`self.K2_GetActorLocation`))
  (bind _impact_point (`self.Impact Point`))
  ;[1 1 1] Rightmouse button - move player
  (`self.AddMovementInput` (`KismetMathLibrary.GetDirectionUnitVector` _returnvalue _impact_point))
  (if (== _returnvalue _impact_point :`ErrorTolerance` 100.0)
    (`KismetSystemLibrary.K2_ClearTimer` null "UpdateMovement")))

(event `SRV_possesSpectator`
  (params (`Spawn Transform Location` :type "Vector Structure") (`Spawn Transform Rotation` :type "Rotator Structure"))
  ;[1 1 1] Posses to spectator
  (bind _returnvalue (`|SpawnActorFromClass` "/Game/PlayerRelated/BP_Spectator.BP_Spectator_C" (`KismetMathLibrary.MakeTransform` `Spawn Transform Location` `Spawn Transform Rotation`) "AdjustIfPossibleButAlwaysSpawn" "OverrideRootScale" null null))
  (`Controller.Possess` (`GameplayStatics.GetPlayerController` 0) _returnvalue))

(event `InputAxisKey|MouseWheelAxis`
  (params (AxisValue :type "Float (single-precision)"))
  ;[1 1 1] Zoomin wheel
  (if (!= AxisValue 0.0)
    (set `self.TargetLength` (`KismetMathLibrary.FClamp` (+ (* AxisValue -350.0) (`SpringArmComponent.TargetArmLength` (`self.SpringArm`))) 550.0 1500.0))))

(event `self.ReceiveTick`
  (params (DeltaSeconds :type "Float (single-precision)"))
  ;[1 1 1] Zoomin wheel
  (set `SpringArmComponent.TargetArmLength` (`KismetMathLibrary.FInterpTo` (`SpringArmComponent.TargetArmLength` (`self.SpringArm`)) (`self.TargetLength`) DeltaSeconds 3.5) (`self.SpringArm`)))

(event `self.ReceiveAnyDamage`
  (params (Damage :type "Float (single-precision)") (DamageType :type "DamageType Object Reference") (InstigatedBy :type "Controller Object Reference") (DamageCauser :type "Actor Object Reference"))
  ;[1 1 1] Remove health
  (`/Game/PlayerRelated/PlayerComponents/BP_PlayerHealth.removeHealth` (`self.BP_PlayerHealth`) Damage))

(event `Key|Q`
  (params (Key :type "Key Structure"))
  (bind _camera (`self.Camera`))
  ;[1 1 1] Press Q to posses
  (:`Pressed`
    (`self.SRV_possesSpectator` (`SceneComponent.K2_GetComponentLocation` _camera) (`SceneComponent.K2_GetComponentRotation` _camera))))

(event `self.BP_PlayerHealth.Event_isDead`
  (bind _camera (`self.Camera`))
  ;[1 1 1] Player died
  (bind _returnvalue (`|SpawnActorFromClass` "/Game/PlayerRelated/BP_Spectator.BP_Spectator_C" (`KismetMathLibrary.MakeTransform` (`SceneComponent.K2_GetComponentLocation` _camera) (`SceneComponent.K2_GetComponentRotation` _camera)) "AdjustIfPossibleButAlwaysSpawn" "OverrideRootScale" null null))
  (`Controller.Possess` (`self.GetController`) _returnvalue)
  (`self.K2_DestroyActor`))

(event `Key|X`
  (params (Key :type "Key Structure"))
  (:`Pressed`
    (`KismetSystemLibrary.PrintString` "CREATING SESSION!")
    (`KismetSystemLibrary.ExecuteConsoleCommand` "open MainLevel?listen" (`GameplayStatics.GetPlayerController` 0))))

(event `Key|Z`
  (params (Key :type "Key Structure"))
  (:`Pressed`
    (`KismetSystemLibrary.PrintString` "FINDING SESSION!")
    (`KismetSystemLibrary.ExecuteConsoleCommand` "open 25.60.130.144" (`GameplayStatics.GetPlayerController` 0))))

(fn `UserConstructionScript`)