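; BP_Spectator is a temporary spectator actor that respawns the player after a short delay.
; On BeginPlay it focuses the game viewport, hides the cursor and starts a timer by function name.
; The timer spawns a BP_MyPlayer at a PlayerStart found by class, has player controller 0 possess it, shows the cursor and destroys the spectator.
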(event `self.ReceiveBeginPlay`
  (`self.SRV_setMouse`)
  (`KismetSystemLibrary.K2_SetTimer` null "SRV_spawnAsPlayer" 2.0))

(event `SRV_setMouse`
  (`WidgetBlueprintLibrary.SetFocusToGameViewport`)
  (set `PlayerController.bShowMouseCursor` false (`GameplayStatics.GetPlayerController` 0)))

(event `SRV_spawnAsPlayer`
  (bind _returnvalue (`GameplayStatics.GetPlayerController` 0))
  (bind _returnvalue_2 (`GameplayStatics.GetActorOfClass` "/Script/Engine.PlayerStart"))
  (bind _returnvalue_3 (`|SpawnActorFromClass` "/Game/PlayerRelated/BP_MyPlayer.BP_MyPlayer_C" (`KismetMathLibrary.MakeTransform` (`self.K2_GetActorLocation` _returnvalue_2)) "AdjustIfPossibleButAlwaysSpawn" "OverrideRootScale" null null))
  (`Controller.Possess` _returnvalue _returnvalue_3)
  (set `PlayerController.bShowMouseCursor` true _returnvalue)
  (`self.K2_DestroyActor`)
  (`KismetSystemLibrary.PrintString` "RESPAWN"))

(fn `UserConstructionScript`)