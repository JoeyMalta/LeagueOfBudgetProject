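; Player component that tracks the player's money and grants passive income over time.
; BeginPlay starts a looping timer through an SRV-prefixed event, which periodically adds a small fixed amount.
; AddMoney and RemoveMoney wrap RPC-prefixed events that adjust CurrentMoney and print the new total, then return CurrentMoney.
; RemoveMoney performs no balance check.
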(event `self.ReceiveBeginPlay`
  (`self.SRV_createTimer`))

(event `SRV_createTimer`
  (`KismetSystemLibrary.K2_SetTimer` null "SRV_incMoney" 1.5 true))

(event `SRV_incMoney`
  (`self.addMoney` 1.0))

(event `RPC_addMoney`
  (params (addedMoney :type "Float (double-precision)"))
  (bind _output_get (set `self.currentMoney` (+ (`self.currentMoney`) addedMoney)))
  (`KismetSystemLibrary.PrintString` (`KismetStringLibrary.Conv_DoubleToString` _output_get) true true (struct :`G` 1.0 :`B` 0.214849 :`A` 1.0) 6.0))

(event `RPC_removeMoney`
  (params (removedMoney :type "Float (double-precision)"))
  (bind _output_get (set `self.currentMoney` (- (`self.currentMoney`) removedMoney)))
  (`KismetSystemLibrary.PrintString` (`KismetStringLibrary.Conv_DoubleToString` _output_get) true true (struct :`R` 1.0 :`G` 0.034265 :`A` 1.0) 6.0))

(fn `addMoney`
  (params (addedMoney :type "Float (double-precision)"))
  (returns (newMoney :type "Float (double-precision)"))
  (`self.RPC_addMoney` addedMoney)
  (return (`self.currentMoney`)))

(fn `removeMoney`
  (params (removedMoney :type "Float (double-precision)"))
  (returns (newMoney :type "Float (double-precision)"))
  (`self.RPC_removeMoney` removedMoney)
  (return (`self.currentMoney`)))