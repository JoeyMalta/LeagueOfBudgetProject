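; Player health component that tracks replicated current health and a dead state for the player.
; AddHealth and RemoveHealth call RPC events that clamp health between zero and MaxHealth, then return the current value.
; Only removal updates Dead, setting it when health equals zero, so healing leaves that flag unchanged.
; The Dead RepNotify fires EventIsDead when true, while the health RepNotify is empty.
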(event `RPC_addHealth`
  (params (addedHealth :type "Float (double-precision)"))
  (set `self.currentHealth` (`KismetMathLibrary.FClamp` (+ (`self.currentHealth`) addedHealth) 0.0 (`self.maxHealth`))))

(event `RPC_removeHealth`
  (params (removedHealth :type "Float (double-precision)"))
  (bind _output_get (set `self.currentHealth` (`KismetMathLibrary.FClamp` (- (`self.currentHealth`) removedHealth) 0.0 (`self.maxHealth`))))
  (set `self.dead` (== _output_get 0.0)))

(fn `addHealth`
  (params (addedHealth :type "Float (double-precision)"))
  (returns (newHealth :type "Float (double-precision)"))
  (`self.RPC_addHealth` addedHealth)
  (return (`self.currentHealth`)))

(fn `isDead`
  (returns (NewParam :type Boolean))
  (return (`self.dead`)))

(fn `OnRep_currentHealth`)

(fn `OnRep_dead`
  (if (`self.dead`)
    (`self.Event_isDead` self)))

(fn `removeHealth`
  (params (removedHealth :type "Float (double-precision)"))
  (returns (newHealth :type "Float (double-precision)"))
  (`self.RPC_removeHealth` removedHealth)
  (return (`self.currentHealth`)))